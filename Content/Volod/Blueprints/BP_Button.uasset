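; BP_Button is an elevator floor button that sends a referenced BP_Lift to its Level height.
; On BeginPlay it creates a WBP_NumButton for its WidgetComponent and passes itself to that widget.
; Interaction plays a click sound and, if the lift's Z differs from Level, calls Up and hides the wall mesh on the linked BP_OpenCloseLift.
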(event EventBeginPlay
  (bind _returnvalue (UserInterface|CreateWidget "/Game/Volod/Blueprints/WBP_NumButton.WBP_NumButton_C"))
  (Variables|/Game/Volod/Blueprints/WBP_NumButton.WBP_NumButton_C|SetRef%20to%20Button _returnvalue self)
  (UserInterface|SetWidget (Variables|Default|GetWidgetComponent) _returnvalue))

(event Collision|EventActorBeginOverlap
  (params (OtherActor :type Actor%20Object%20Reference)))

(event EventTick
  (params (DeltaSeconds :type Float%20%28single-precision%29)))

(event EventInteraction
  (bind _asbp_lift (Utilities|Casting|CastToBP_Lift (Variables|Default|GetLift)))
  (Audio|PlaySound2D "/Game/Volod/Sound/jg-032316-sfx-elevator-button.jg-032316-sfx-elevator-button" 1.0 1.0 0.0 0 0)
  (if (!= (.z (Transformation|GetActorLocation _asbp_lift)) (Variables|Default|Getlevel))
    (Default|Up _asbp_lift (Variables|Default|Getlevel))
    (bind _asbp_open_close_lift (Utilities|Casting|CastToBP_OpenCloseLift (Variables|Default|GetOpenDoorButton)))
    (Rendering|SetVisibility (Variables|/Game/Volod/Blueprints/BP_OpenCloseLift.BP_OpenCloseLift_C|GetWall_400x200 _asbp_open_close_lift) false false)))

(fn ConstructionScript)