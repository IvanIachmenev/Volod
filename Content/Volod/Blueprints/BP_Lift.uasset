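; BP_Lift is an elevator actor that changes height on an Up call and has a door that slides vertically.
; Up waits, then plays a timeline whose update sets actor Z directly to the requested level, as the Lerp alpha is fixed at zero.
; The same update chains delays to open and later close the door, then stores the new level.
; The OpenAnimation timeline drives the door mesh's relative Z, playing forward to open and reversing to close.
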(event Custom|Up
  (params (Level :type Float%20%28double-precision%29))
  (bind _returnvalue (Transformation|GetActorLocation))
  (Variables|Default|SetLevel_0 Level)
  (Utilities|FlowControl|Delay 1e+01)
  (Timeline|Timeline Play
    (:Update
      (Transformation|SetActorLocation (Math|Vector|MakeVector (.x _returnvalue) (.y _returnvalue) (Math|Float|Lerp (Variables|Default|GetLevel_0) (.z _returnvalue) 0.0)) false false)
      (Utilities|FlowControl|Delay 8.0)
      (CallFunction|OpenDoor)
      (Utilities|FlowControl|Delay 6.0)
      (CallFunction|CloseDoor)
      (Variables|Default|SetLevel (Variables|Default|GetLevel_0)))))

(event Custom|OpenDoor
  (bind _doormesh (Variables|Default|GetDoorMesh))
  (bind _relativelocation (Variables|/Script/Engine.SceneComponent|GetRelativeLocation _doormesh))
  (bind _openclose (Timeline|OpenAnimation Play)
    (:Update
      (Transformation|SetRelativeLocation (Variables|Default|GetDoorMesh) (Math|Vector|MakeVector (.x (Math|Vector|Lerp(Vector) (Math|Vector|MakeVector (.x _relativelocation) (.y _relativelocation) 75.428574) (Math|Vector|MakeVector (.x _relativelocation) (.y _relativelocation) 127.0) _openclose)) (.y (Math|Vector|Lerp(Vector) (Math|Vector|MakeVector (.x _relativelocation) (.y _relativelocation) 75.428574) (Math|Vector|MakeVector (.x _relativelocation) (.y _relativelocation) 127.0) _openclose)) (.z (Math|Vector|Lerp(Vector) (Math|Vector|MakeVector (.x _relativelocation) (.y _relativelocation) 75.428574) (Math|Vector|MakeVector (.x _relativelocation) (.y _relativelocation) 127.0) _openclose))) false false))))

(event Custom|CloseDoor
  (bind _doormesh (Variables|Default|GetDoorMesh))
  (bind _relativelocation (Variables|/Script/Engine.SceneComponent|GetRelativeLocation _doormesh))
  (bind _openclose (Timeline|OpenAnimation Reverse)
    (:Update
      (Transformation|SetRelativeLocation (Variables|Default|GetDoorMesh) (Math|Vector|MakeVector (.x (Math|Vector|Lerp(Vector) (Math|Vector|MakeVector (.x _relativelocation) (.y _relativelocation) 75.428574) (Math|Vector|MakeVector (.x _relativelocation) (.y _relativelocation) 127.0) _openclose)) (.y (Math|Vector|Lerp(Vector) (Math|Vector|MakeVector (.x _relativelocation) (.y _relativelocation) 75.428574) (Math|Vector|MakeVector (.x _relativelocation) (.y _relativelocation) 127.0) _openclose)) (.z (Math|Vector|Lerp(Vector) (Math|Vector|MakeVector (.x _relativelocation) (.y _relativelocation) 75.428574) (Math|Vector|MakeVector (.x _relativelocation) (.y _relativelocation) 127.0) _openclose))) false false))))

(event EventBeginPlay
  (Variables|Default|SetLevel (.z (Transformation|GetActorLocation))))

(event Collision|EventActorBeginOverlap
  (params (OtherActor :type Actor%20Object%20Reference)))

(fn ConstructionScript)