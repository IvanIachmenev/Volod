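; BP_OpenCloseLift is an interactable lift call control that brings a referenced BP_Lift to its Level and cycles the door.
; Interaction plays a button sound and, if the lift's Level differs, hides Wall400x200, teleports the lift to Level as its Z, then pauses.
; It then calls OpenDoor and CloseDoor on timed delays and makes the wall visible again.
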(event EventBeginPlay
  (|CallParentFunction) ; This node is disabled and will not be called.\nDrag off pins to build functionality.
)

(event Collision|EventActorBeginOverlap
  (params (OtherActor :type Actor%20Object%20Reference))
  (|CallParentFunction OtherActor) ; This node is disabled and will not be called.\nDrag off pins to build functionality.
)

(event EventTick
  (params (DeltaSeconds :type Float%20%28single-precision%29))
  (|CallParentFunction DeltaSeconds) ; This node is disabled and will not be called.\nDrag off pins to build functionality.
)

(event EventInteraction
  (bind _lift (Variables|Default|GetLift))
  (bind _returnvalue (Transformation|GetActorLocation _lift))
  (bind _asbp_lift (Utilities|Casting|CastToBP_Lift (Variables|Default|GetLift)))
  (Audio|PlaySound2D "/Game/Volod/Sound/jg-032316-sfx-elevator-button.jg-032316-sfx-elevator-button" 1.0 1.0 0.0 0 0)
  (if (== (Variables|/Game/Volod/Blueprints/BP_Lift.BP_Lift_C|GetLevel _asbp_lift) (Variables|Default|Getlevel))
    _
    (else
      (Rendering|SetVisibility (Variables|Default|GetWall_400x200) false false)
      (Transformation|SetActorLocation (Variables|Default|GetLift) (Math|Vector|MakeVector (.x _returnvalue) (.y _returnvalue) (Variables|Default|Getlevel)) false false)
      (Utilities|FlowControl|Delay 2.0)))
  (Default|OpenDoor _asbp_lift)
  (Utilities|FlowControl|Delay 6.0)
  (Default|CloseDoor _asbp_lift)
  (Utilities|FlowControl|Delay 6.0)
  (Rendering|SetVisibility (Variables|Default|GetWall_400x200) true false))

(fn ConstructionScript
  (|CallParentFunction))